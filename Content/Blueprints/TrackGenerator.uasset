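; Spline-driven track generator actor that builds a road with optional left and right guard rails in its construction script.
; It resizes a per-point road data array to match the spline points, filling new entries with defaults.
; For each segment between consecutive points, BuildTrackElement adds spline mesh components, interpolating bank, width and thickness from both end points, with toggleable collision.
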(event EventBeginPlay)

(event Collision|EventActorBeginOverlap
  (params (OtherActor :type Actor%20Object%20Reference)))

(event EventTick
  (params (DeltaSeconds :type Float%20%28single-precision%29)))

(fn ConstructionScript
  (bind _roaddataarray (Variables|Default|GetRoadDataArray))
  (Utilities|FlowControl|Sequence
    (:then_0
      (Variables|Default|SetNumber%20of%20SplinePoints (Class|SplineComponent|GetNumSplinePoints (Variables|Default|GetSpline))))
    (:then_1
      (Math|Integer|CompareInt (Utilities|Array|Length (Variables|Default|GetRoadDataArray)) (Variables|Default|GetNumber%20of%20SplinePoints) :!label _label
        (:>
          (Utilities|Array|RemoveIndex _roaddataarray (Utilities|Array|LastIndex _roaddataarray))
          (goto _label))
        (:<
          (Utilities|Array|Add (Variables|Default|GetRoadDataArray) (Variables|Default|GetRoadMeshDefaults))
          (goto _label))))
    (:then_2
      (for _index (range 0 (- (Variables|Default|GetNumber%20of%20SplinePoints) 2))
        (Variables|Default|SetCurrentLoopIndex _index)
        (Variables|Default|SetDrawLeftGuardRail (.leftguardrail (Utilities|Array|Get(acopy) (Variables|Default|GetRoadDataArray) (Variables|Default|GetCurrentLoopIndex))))
        (Variables|Default|SetDrawRightGuardRail (.rightguardrail (Utilities|Array|Get(acopy) (Variables|Default|GetRoadDataArray) (Variables|Default|GetCurrentLoopIndex))))
        (Utilities|FlowControl|Sequence
          (:then_0
            (CallFunction|BuildTrackElement (Variables|Default|GetCurrentLoopIndex) (Variables|Default|GetRoadMesh)))
          (:then_1
            (if (Variables|Default|GetDrawLeftGuardRail)
              (CallFunction|BuildTrackElement (Variables|Default|GetCurrentLoopIndex) (Variables|Default|GetLeftGuardRailMesh))))
          (:then_2
            (if (Variables|Default|GetDrawRightGuardRail)
              (CallFunction|BuildTrackElement (Variables|Default|GetCurrentLoopIndex) (Variables|Default|GetRightGuardRailMesh)))))))
    (:then_3)))

(fn BuildTrackElement
  (params (LoopIndex :type Integer) (TrackElementMesh :type Static%20Mesh%20Object%20Reference))
  (LocalVariables|SetLocal_CurrentLoopIndex LoopIndex)
  (LocalVariables|SetLocal_NextLoopIndex (Math|Integer|%(Integer) (+ LoopIndex 1) (Variables|Default|GetNumber%20of%20SplinePoints)))
  (LocalVariables|SetLocal_TrackElementMesh TrackElementMesh)
  (Utilities|FlowControl|Sequence
    (:then_0
      (LocalVariables|SetLocal_startLocation (.LocalLocation (Class|SplineComponent|GetLocalLocationandTangentatSplinePoint (Variables|Default|GetSpline) (LocalVariables|GetLocal_CurrentLoopIndex))))
      (LocalVariables|SetLocal_StartTangent (.LocalTangent (Class|SplineComponent|GetLocalLocationandTangentatSplinePoint (Variables|Default|GetSpline) (LocalVariables|GetLocal_CurrentLoopIndex))))
      (LocalVariables|SetLocal_EndLocation (.LocalLocation (Class|SplineComponent|GetLocalLocationandTangentatSplinePoint (Variables|Default|GetSpline) (LocalVariables|GetLocal_NextLoopIndex))))
      (LocalVariables|SetLocal_EndTangent (.LocalTangent (Class|SplineComponent|GetLocalLocationandTangentatSplinePoint (Variables|Default|GetSpline) (LocalVariables|GetLocal_NextLoopIndex))))
      (LocalVariables|SetLocal_StartRoll (.trackbank (Utilities|Array|Get(acopy) (Variables|Default|GetRoadDataArray) (LocalVariables|GetLocal_CurrentLoopIndex))))
      (LocalVariables|SetLocal_StartScale (Math|Vector2D|MakeVector2D (.trackwidth (Utilities|Array|Get(acopy) (Variables|Default|GetRoadDataArray) (LocalVariables|GetLocal_CurrentLoopIndex))) (.trackthickness (Utilities|Array|Get(acopy) (Variables|Default|GetRoadDataArray) (LocalVariables|GetLocal_CurrentLoopIndex)))))
      (LocalVariables|SetLocal_EndRoll (.trackbank (Utilities|Array|Get(acopy) (Variables|Default|GetRoadDataArray) (LocalVariables|GetLocal_NextLoopIndex))))
      (LocalVariables|SetLocal_EndScale (Math|Vector2D|MakeVector2D (.trackwidth (Utilities|Array|Get(acopy) (Variables|Default|GetRoadDataArray) (LocalVariables|GetLocal_NextLoopIndex))) (.trackthickness (Utilities|Array|Get(acopy) (Variables|Default|GetRoadDataArray) (LocalVariables|GetLocal_NextLoopIndex))))))
    (:then_1
      (bind _returnvalue (AddComponent|AddSplineMeshComponent false))
      (LocalVariables|SetLocal_CurrentSplineMesh _returnvalue)
      (Components|StaticMesh|SetStaticMesh (LocalVariables|GetLocal_CurrentSplineMesh) (LocalVariables|GetLocal_TrackElementMesh))
      (SplineMesh|SetStartandEnd (LocalVariables|GetLocal_CurrentSplineMesh) (LocalVariables|GetLocal_startLocation) (LocalVariables|GetLocal_StartTangent) (LocalVariables|GetLocal_EndLocation) (LocalVariables|GetLocal_EndTangent) :!class /Script/Engine.SplineMeshComponent)
      (Class|SplineMeshComponent|SetStartRoll (LocalVariables|GetLocal_CurrentSplineMesh) (LocalVariables|GetLocal_StartRoll))
      (Class|SplineMeshComponent|SetEndRoll (LocalVariables|GetLocal_CurrentSplineMesh) (LocalVariables|GetLocal_EndRoll))
      (SplineMesh|SetStartScale (LocalVariables|GetLocal_CurrentSplineMesh) (LocalVariables|GetLocal_StartScale) :!class /Script/Engine.SplineMeshComponent)
      (SplineMesh|SetEndScale (LocalVariables|GetLocal_CurrentSplineMesh) (LocalVariables|GetLocal_EndScale) :!class /Script/Engine.SplineMeshComponent)
      (Collision|SetCollisionEnabled (LocalVariables|GetLocal_CurrentSplineMesh) (select (Variables|Default|GetCollisions) "QueryAndPhysics" "NoCollision")))))